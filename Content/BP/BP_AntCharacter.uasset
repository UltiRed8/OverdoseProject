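; Player ant character Blueprint that handles saved input bindings, item aiming and jump audio.
; BeginPlay hooks up two world life-bar widgets and rebuilds the input mapping context from the "Inputs" remap save.
; While aiming, Tick caches the current item and rotates it to match the camera; a jump counter and DoOnce drive jump, double-jump and landing sounds.
; The construction script attaches per-item arrow components to the right wrist socket.
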(event `self.ReceiveBeginPlay`
  (bind _mappings (`InputMappingContext.Mappings` (`self.IMC`)))
  (`|ExecutionSequence`
    (:`then_0`
      (bind _asw_world_life_bar (cast `/Game/Widget/Menu/UI_Player/W_WorldLifeBar` (`WidgetComponent.GetWidget` (`self.widget`))))
      (`/Game/Widget/Menu/UI_Player/W_WorldLifeBar.SetCustomOwner` _asw_world_life_bar self)
      (bind _asw_world_life_bar_2 (cast `/Game/Widget/Menu/UI_Player/W_WorldLifeBar` (`WidgetComponent.GetWidget` (`self.widget2`))))
      (`/Game/Widget/Menu/UI_Player/W_WorldLifeBar.SetCustomOwner` _asw_world_life_bar_2 self)
      (`GameplayStatics.DoesSaveGameExist` "Inputs")
      (bind _returnvalue (`GameplayStatics.LoadGameFromSlot` "Inputs"))
      (bind _asremap_save (cast `/Game/Data/RemapSave` _returnvalue))
      (`KismetArrayLibrary.Array_Clear` _mappings)
      (for _array_element (`/Game/Data/RemapSave.mappings` _asremap_save)
        (`KismetArrayLibrary.Array_Add` _mappings _array_element))
      (`self.SetInputMappingContext` (`self.IMC`)))
    (:`then_1`
      (add `self.onJump` (delegate `SoundJumping`)))))

(event `SoundJumping`
  (bind _jumps (`self.Jumps`))
  (`|ExecutionSequence`
    (:`then_0`
      (switch `int` _jumps
        (:`0`
          (`AudioComponent.Play` (`self.AudioJump`) 0.0))
        (:`1`
          (`AudioComponent.Play` (`self.AudioDoubleJump`) 0.0))))
    (:`then_1`
      (`/Engine/EditorBlueprintResources/StandardMacros.IncrementInt` _jumps))))

(event `self.ReceiveTick`
  (params (DeltaSeconds :type "Float (single-precision)"))
  (bind _holdingitem (`self.HoldingItem`))
  (`|ExecutionSequence`
    (:`then_0`
      (bind _returnvalue (`self.IsAiming`))
      (if _returnvalue
        (`/Engine/EditorBlueprintResources/StandardMacros.IsValid` _holdingitem
          (:`Is Valid`
            _)
          (:`Is Not Valid`
            (bind _returnvalue_2 (`self.GetItem`))
            (`/Engine/EditorBlueprintResources/StandardMacros.IsValid` _returnvalue_2
              (:`Is Valid`
                (set `self.HoldingItem` _returnvalue_2)))))
        (`self.K2_SetActorRotation` (`self.HoldingItem`) (`SceneComponent.K2_GetComponentRotation` (`self.camera`)) false)
        (else
          (`/Engine/EditorBlueprintResources/StandardMacros.IsValid` _holdingitem
            (:`Is Valid`
              (set `self.HoldingItem` null))))))
    (:`then_1`
      (if (`NavMovementComponent.IsFalling` (`self.CharacterMovement`))
        (goto _label :!via `Reset`)
        (else
          (`/Engine/EditorBlueprintResources/StandardMacros.DoOnce` false :!label _label
            (:`Completed`
              (set `self.Jumps` 0)
              (`AudioComponent.Play` (`self.AudioLanding`) 0.0))))))))

(fn `UserConstructionScript`
  (`SceneComponent.K2_AttachToComponent` (`self.healArrow`) (`self.Mesh`) "R_wrist" "KeepRelative" "KeepRelative" "KeepRelative" true)
  (`SceneComponent.K2_AttachToComponent` (`self.teleporterArrow`) (`self.Mesh`) "R_wrist" "KeepRelative" "KeepRelative" "KeepRelative" true)
  (`SceneComponent.K2_AttachToComponent` (`self.bazookaArrow`) (`self.Mesh`) "R_wrist" "KeepRelative" "KeepRelative" "KeepRelative" true)
  (`SceneComponent.K2_AttachToComponent` (`self.rubiksCubeArrow`) (`self.Mesh`) "R_wrist" "KeepRelative" "KeepRelative" "KeepRelative" true)
  (`SceneComponent.K2_AttachToComponent` (`self.rasputinArrow`) (`self.Mesh`) "R_wrist" "KeepRelative" "KeepRelative" "KeepRelative" true)
  (`SceneComponent.K2_AttachToComponent` (`self.fallingMokiaArrow`) (`self.Mesh`) "R_wrist" "KeepRelative" "KeepRelative" "KeepRelative" true))