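; BP_GhostAntCharacter is the ghost ant character Blueprint, handling its sound feedback for spawning, movement and items.
; A 2D sound plays from a bound OnSpawn event, and another plays each time HasItem turns true.
; Tick checks velocity and uses paired DoOnce gates to play or reverse the Progress timeline on movement changes, fading the Audio component's volume.
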(event `onSpawn_Event`
  (`GameplayStatics.PlaySound2D` null 1.0 1.0 0.0 null null))

(event `self.ReceiveBeginPlay`
  (add `self.onSpawn` (delegate `onSpawn_Event`)))

(event `self.ReceiveTick`
  (params (DeltaSeconds :type "Float (single-precision)"))
  (bind (_returnvalue_x _returnvalue_y _returnvalue_z) (`KismetMathLibrary.BreakVector` (`self.GetVelocity`)))
  (`|ExecutionSequence`
    (:`then_0`
      (if (> (+ (`KismetMathLibrary.Abs` _returnvalue_x) (`KismetMathLibrary.Abs` _returnvalue_y) (`KismetMathLibrary.Abs` _returnvalue_z)) 0.0)
        (`|ExecutionSequence`
          (:`then_0`
            (`/Engine/EditorBlueprintResources/StandardMacros.DoOnce` false :!label _label
              (:`Completed`
                (bind (_direction _value) (`Timeline|Progress` :!label _label_2)
                  (:`Update`
                    (`AudioComponent.SetVolumeMultiplier` (`self.Audio`) _value))))))
          (:`then_1`
            (goto _label_3 :!via `Reset`)))
        (else
          (`|ExecutionSequence`
            (:`then_0`
              (`/Engine/EditorBlueprintResources/StandardMacros.DoOnce` false :!label _label_3
                (:`Completed`
                  (goto _label_2 :!via `Reverse`))))
            (:`then_1`
              (goto _label :!via `Reset`))))))
    (:`then_1`
      (bind _returnvalue (`self.HasItem`))
      (if _returnvalue
        (`/Engine/EditorBlueprintResources/StandardMacros.DoOnce` false :!label _label_4
          (:`Completed`
            (`GameplayStatics.PlaySound2D` null 1.0 1.0 0.0 null null)))
        (else
          (goto _label_4 :!via `Reset`))))))

(fn `UserConstructionScript`)