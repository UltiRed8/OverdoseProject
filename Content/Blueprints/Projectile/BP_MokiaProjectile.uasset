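; BP_MokiaProjectile is the Mokia projectile, handling audio and chat feedback when it explodes.
; On BeginPlay it binds its explosion handler to the ExplosableComponent.
; On explosion it spawns BP_AudioActors for a nova sound at the mesh and an explosion sound at the actor location.
; It then passes the name of each BP_AntCharacter within the component's radius to the chat subsystem as damaged by Mokia.
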(event `self.ReceiveBeginPlay`
  (add `ExplosableComponent.onExplosion` (`self.explosableComponent`) (delegate `onExplosion_Event`)))

(event `onExplosion_Event`
  (`|SpawnActorFromClass` "/Game/Audio/BP_AudioActor.BP_AudioActor_C" (`KismetMathLibrary.MakeTransform` (`SceneComponent.K2_GetComponentLocation` (`self.mesh`))) "Undefined" "MultiplyWithRoot" null "/Game/Audio/Sounds/Objects/Weapons/Mokia/SA_Mokia_Feedback_Nova_ROU.SA_Mokia_Feedback_Nova_ROU" null)
  (`|SpawnActorFromClass` "/Game/Audio/BP_AudioActor.BP_AudioActor_C" (`KismetMathLibrary.MakeTransform` (`self.K2_GetActorLocation`)) "Undefined" "MultiplyWithRoot" null "/Game/Audio/Sounds/Objects/Weapons/Mokia/SA_Mokia_Feedback_Explosion1_ROU.SA_Mokia_Feedback_Explosion1_ROU" null)
  (bind _returnvalue (`ExplosableComponent.GetActorInRadius` (`self.explosableComponent`)))
  (for _array_element _returnvalue
    (bind _asbp_ant_character (cast `/Game/BP/BP_AntCharacter` _array_element))
    (bind _returnvalue_2 (`AntCharacter.GetName` _asbp_ant_character))
    (`ChatSubsystem.DamageByMokia` (subsystem `ChatSubsystem`) _returnvalue_2)))

(fn `UserConstructionScript`)