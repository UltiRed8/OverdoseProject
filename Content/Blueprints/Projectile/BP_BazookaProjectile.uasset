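; Bazooka projectile that reacts to its explosion with confetti, sound and chat reporting of the ants caught in the blast.
; On BeginPlay it binds to its ExplosableComponent's explosion event, which spawns effect and audio actors at the mesh location.
; If the projectile owner is an ant character, each ant in the component's radius is reported to ChatSubsystem as bazooka damage, with sender and receiver names.
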(event `self.ReceiveBeginPlay`
  (add `ExplosableComponent.onExplosion` (`self.explosableComponent`) (delegate `onExplosion`)))

(event `onExplosion`
  (bind _returnvalue (`SceneComponent.K2_GetComponentLocation` (`self.mesh`)))
  (`|SpawnActorFromClass` "/Game/Blueprints/Actors/BP_EffectActor.BP_EffectActor_C" (`KismetMathLibrary.MakeTransform` _returnvalue) "AlwaysSpawn" "MultiplyWithRoot" null "/Game/Graph/FX/NS_Confetti_Explosion.NS_Confetti_Explosion" null)
  (`|SpawnActorFromClass` "/Game/Audio/BP_AudioActor.BP_AudioActor_C" (`KismetMathLibrary.MakeTransform` _returnvalue) "Undefined" "MultiplyWithRoot" null "/Game/Audio/Sounds/Objects/Weapons/Bazooka/SA_Bazooka_Feedback_Explosion_MOI.SA_Bazooka_Feedback_Explosion_MOI" null)
  (bind _returnvalue_2 (`self.GetProjectileOwner`))
  (bind _asbp_ant_character (cast `/Game/BP/BP_AntCharacter` _returnvalue_2))
  (bind _returnvalue_3 (`AntCharacter.GetName` _asbp_ant_character))
  (bind _returnvalue_4 (`ExplosableComponent.GetActorInRadius` (`self.explosableComponent`)))
  (for _array_element _returnvalue_4
    (bind _asbp_ant_character_2 (cast `/Game/BP/BP_AntCharacter` _array_element))
    (bind _returnvalue_5 (`AntCharacter.GetName` _asbp_ant_character_2))
    (`ChatSubsystem.DamageByBazooka` (subsystem `ChatSubsystem`) _returnvalue_3 _returnvalue_5)))

(fn `UserConstructionScript`)