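; BP_RasputinProjectile is an exploding projectile that reports the ants caught in its Rasputin blast.
; On BeginPlay it binds a handler to its ExplosableComponent's explosion event.
; On explosion, it spawns audio and Niagara effect actors at the mesh location.
; It then queries the component for actors in radius and passes each BP_AntCharacter's name to the ChatSubsystem's DamageByRasputin.
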(event `self.ReceiveBeginPlay`
  (add `ExplosableComponent.onExplosion` (`self.explosableComponent`) (delegate `onExplosion_Event`)))

(event `onExplosion_Event`
  (bind _returnvalue (`SceneComponent.K2_GetComponentLocation` (`self.mesh`)))
  (`|SpawnActorFromClass` "/Game/Audio/BP_AudioActor.BP_AudioActor_C" (`KismetMathLibrary.MakeTransform` _returnvalue) "Undefined" "MultiplyWithRoot" null "/Game/Audio/Sounds/Objects/Weapons/Rasputin/SA_Rasputin_Feedback_Explosion_JAC_V3.SA_Rasputin_Feedback_Explosion_JAC_V3" null)
  (`|SpawnActorFromClass` "/Game/Blueprints/Actors/BP_EffectActor.BP_EffectActor_C" (`KismetMathLibrary.MakeTransform` _returnvalue) "AlwaysSpawn" "MultiplyWithRoot" null "/Game/Graph/FX/NS_Explosion_Test_2.NS_Explosion_Test_2" null)
  (bind _returnvalue_2 (`ExplosableComponent.GetActorInRadius` (`self.explosableComponent`)))
  (for _array_element _returnvalue_2
    (bind _asbp_ant_character (cast `/Game/BP/BP_AntCharacter` _array_element))
    (bind _returnvalue_3 (`AntCharacter.GetName` _asbp_ant_character))
    (`ChatSubsystem.DamageByRasputin` (subsystem `ChatSubsystem`) _returnvalue_3)))

(fn `UserConstructionScript`)