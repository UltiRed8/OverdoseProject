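; BP_Mine is a Rubik's Cube mine that reacts to ant characters and explodes through its ExplosableComponent.
; The first ant overlap activates its Niagara effect, hides the root component and plays an activation sound, guarded by DoOnce.
; The component's explosion event spawns effect and audio actors, then reports ants in the blast radius by name to ChatSubsystem as Rubik's Cube damage.
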(event `self.ReceiveBeginPlay`
  (add `ExplosableComponent.onExplosion` (`self.explosableComponent`) (delegate `onExplosion`)))

(event `onExplosion`
  (bind _returnvalue (`self.K2_GetActorLocation`))
  (`|SpawnActorFromClass` "/Game/Blueprints/Actors/BP_EffectActor.BP_EffectActor_C" (`KismetMathLibrary.MakeTransform` _returnvalue) "AlwaysSpawn" "MultiplyWithRoot" null "/Game/Graph/FX/NS_Explosion_Test_2.NS_Explosion_Test_2" null)
  (`|SpawnActorFromClass` "/Game/Audio/BP_AudioActor.BP_AudioActor_C" (`KismetMathLibrary.MakeTransform` _returnvalue) "Undefined" "MultiplyWithRoot" null "/Game/Audio/Sounds/Objects/Weapons/RubiksCube/SA_Rubik_Feedback_Explosion_ROU.SA_Rubik_Feedback_Explosion_ROU" null)
  (bind _returnvalue_2 (`ExplosableComponent.GetActorInRadius` (`self.explosableComponent`)))
  (for _array_element _returnvalue_2
    (bind _asbp_ant_character (cast `/Game/BP/BP_AntCharacter` _array_element))
    (bind _returnvalue_3 (`AntCharacter.GetName` _asbp_ant_character))
    (`ChatSubsystem.DamageByRubiksCube` (subsystem `ChatSubsystem`) _returnvalue_3)))

(event `self.ReceiveActorBeginOverlap`
  (params (OtherActor :type "Actor Object Reference"))
  (`|ExecutionSequence`
    (:`then_0`
      (cast `/Game/BP/BP_AntCharacter` OtherActor)
      (`/Engine/EditorBlueprintResources/StandardMacros.DoOnce` false
        (:`Completed`
          (`ActorComponent.Activate` (`self.Niagara`) false)
          (`SceneComponent.SetVisibility` (`self.RootComponent`) false false)
          (`|SpawnActorFromClass` "/Game/Audio/BP_AudioActor.BP_AudioActor_C" (`KismetMathLibrary.MakeTransform` (`self.K2_GetActorLocation`)) "Undefined" "MultiplyWithRoot" null "/Game/Audio/Sounds/Objects/Weapons/Mokia/SA_Rubik_Feedback_Activation_4_ROU.SA_Rubik_Feedback_Activation_4_ROU" null))))))

(fn `UserConstructionScript`)