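; Bazooka weapon item that spawns an explosion effect actor at its Arrow's location when used.
; BeginPlay binds the item-used event, which spawns BP_EffectActor with a test Niagara explosion.
; The construction script tiles collision-free, glowing red spline meshes along the Spline, with tangents clamped to section length.
; Section length can follow actor X scale, and MustBeFullLengthMeshes adds one extra segment for the remainder.
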(event `self.ReceiveBeginPlay`
  (add `Item.onItemUsed` (delegate `onItemUsed_Event`)))

(event `onItemUsed_Event`
  (`|SpawnActorFromClass` "/Game/Blueprints/Actors/BP_EffectActor.BP_EffectActor_C" (`KismetMathLibrary.MakeTransform` (`SceneComponent.K2_GetComponentLocation` (`self.Arrow`))) "AlwaysSpawn" "MultiplyWithRoot" null "/Game/Graph/FX/NS_Explosion_Test_1.NS_Explosion_Test_1" null))

(fn `UserConstructionScript`
  (bind _returnvalue_x (`KismetMathLibrary.BreakVector` (`self.GetActorScale3D`)))
  (bind _spline (`self.spline`))
  (bind _spline_2 (`self.spline`))
  (bind _returnvalue (* (`self.LoopIndex`) (`self.SectionLength`)))
  (bind _returnvalue_2 (* (+ (`self.LoopIndex`) 1) (`self.SectionLength`)))
  (if (`self.AllowScaling`)
    (set `self.SectionLength` (* _returnvalue_x 100.0)))
  (if (`self.MustBeFullLengthMeshes`)
    (for _index (range (+ (`KismetMathLibrary.FTrunc` (/ (`SplineComponent.GetSplineLength` (`self.spline`)) (`self.SectionLength`))) 1))
      (set `self.LoopIndex` _index)
      (bind _returnvalue_3 (`AddComponent|NODE_AddSplineMeshComponent-0` :!label _label))
      (`StaticMeshComponent.SetStaticMesh` _returnvalue_3 (`self.SplineMesh`))
      (`PrimitiveComponent.SetMaterial` _returnvalue_3 0 "/Game/Materials/MI_GlowRed.MI_GlowRed")
      (`SplineMeshComponent.SetForwardAxis` _returnvalue_3 "X" true)
      (`SplineMeshComponent.SetStartAndEnd` _returnvalue_3 (`SplineComponent.GetLocationAtDistanceAlongSpline` _spline _returnvalue "Local") (`KismetMathLibrary.ClampVectorSize` (`SplineComponent.GetTangentAtDistanceAlongSpline` _spline _returnvalue "Local") 0.0 (`self.SectionLength`)) (`SplineComponent.GetLocationAtDistanceAlongSpline` _spline_2 _returnvalue_2 "Local") (`KismetMathLibrary.ClampVectorSize` (`SplineComponent.GetTangentAtDistanceAlongSpline` _spline_2 _returnvalue_2 "Local") 0.0 (`self.SectionLength`)) true)
      (`PrimitiveComponent.SetCollisionEnabled` _returnvalue_3 "NoCollision"))
    (else
      (for _index_2 (range (`KismetMathLibrary.FTrunc` (/ (`SplineComponent.GetSplineLength` (`self.spline`)) (`self.SectionLength`))))
        (set `self.LoopIndex` _index_2)
        (goto _label)))))