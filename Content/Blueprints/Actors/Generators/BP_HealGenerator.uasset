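; BP_HealGenerator is a generator actor, named for healing, whose Blueprint handles its audio feedback.
; On BeginPlay it binds to its OnGenerated dispatcher and its ExplosableComponent's explosion event.
; Each generation activates three audio components.
; An explosion spawns a separate BP_AudioActor at the generator's location to play the explosion sound.
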(event `onExplosion`
  (`|SpawnActorFromClass` "/Game/Audio/BP_AudioActor.BP_AudioActor_C" (`KismetMathLibrary.MakeTransform` (`self.K2_GetActorLocation`)) "Undefined" "MultiplyWithRoot" null "/Game/Audio/Sounds/Objects/Generator/SA_Generator_Feedback_Explosion2_LIM.SA_Generator_Feedback_Explosion2_LIM" null))

(event `self.ReceiveBeginPlay`
  (add `self.onGenerated` (delegate `onGenerated_Event`))
  (add `ExplosableComponent.onExplosion` (`self.explosableComponent`) (delegate `onExplosion`)))

(event `onGenerated_Event`
  (`ActorComponent.Activate` (`self.Audio1`) false)
  (`ActorComponent.Activate` (`self.Audio2`) false)
  (`ActorComponent.Activate` (`self.Audio3`) false))

(fn `UserConstructionScript`)