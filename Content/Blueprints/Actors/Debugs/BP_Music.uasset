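; BP_Music is a level actor that plays adaptive music reflecting which team leads in life.
; After each player end action, it compares team lives and switches to Neutral on a tie, or to the leader's Disco or Sport theme, inferred from the first team's mesh.
; Timelines crossfade three audio components, each given a random track.
; A looping delay fires MusicSubsystem beat triggers at the current theme's BPM.
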(event `self.ReceiveBeginPlay`
  (if (not (`self.Disabled`))
    (add `GameSubsystem.onPlayerEndAction` (subsystem `GameSubsystem`) (delegate `onPlayerEndAction_Event`))
    (bind _returnvalue (`TeamInfoSubsystem.GetTeamDatas` (subsystem `TeamInfoSubsystem`)))
    (bind _output_mesh (break `TeamData` (`|GetArrayItem` _returnvalue)))
    (set `self.isFirstTeamDisco` (== _output_mesh "/Game/Graph/Chara/Fourmi_disco_fini.Fourmi_disco_fini"))
    (`self.SwitchMusic`)
    (`KismetSystemLibrary.Delay` (/ 1.0 (/ (`self.CurrentBPM`) 60)) :!label _label)
    (`MusicSubsystem.onBeatTrigger` (subsystem `MusicSubsystem`))
    (goto _label)))

(event `onPlayerEndAction_Event`
  (bind _returnvalue (subsystem `GameSubsystem`))
  (bind _state (`self.State`))
  (bind _returnvalue_2 (`GameSubsystem.GetLifeTeam1` _returnvalue))
  (bind _returnvalue_3 (`GameSubsystem.GetLifeTeam2` _returnvalue))
  (if (== _returnvalue_2 _returnvalue_3)
    (if (!= _state 0)
      (set `self.State` 0)
      (`self.SwitchMusic` :!label _label_2))
    (elif (> _returnvalue_2 _returnvalue_3)
      (if (!= _state 1)
        (set `self.State` 1)
        (goto _label_2))
      (elif (!= _state 2)
        (set `self.State` 2)
        (goto _label_2)))))

(event `GoNeutral`
  (`AudioComponent.SetSound` (`self.Neutral`) (`KismetArrayLibrary.Array_Random` (`self.NeutralMusics`)))
  (`|ExecutionSequence`
    (:`then_0`
      (bind (_direction _status) (`Timeline|NeutralProgress` :!label _label_3)
        (:`Update`
          (`AudioComponent.SetVolumeMultiplier` (`self.Neutral`) _status))))
    (:`then_1`
      (bind (_direction_2 _status_2) (`Timeline|DiscoProgress` :!via `Reverse` :!label _label_4)
        (:`Update`
          (`AudioComponent.SetVolumeMultiplier` (`self.Disco`) _status_2))))
    (:`then_2`
      (bind (_direction_3 _status_3) (`Timeline|SportProgress` :!via `Reverse` :!label _label_5)
        (:`Update`
          (`AudioComponent.SetVolumeMultiplier` (`self.Sport`) _status_3))))))

(event `SwitchMusic`
  (bind _isfirstteamdisco (`self.isFirstTeamDisco`))
  (switch `int` (`self.State`)
    (:`0`
      (`self.GoNeutral`)
      (set `self.CurrentBPM` (`self.NeutralBPM`)))
    (:`1`
      (if _isfirstteamdisco
        (`self.GoDisco` :!label _label_6)
        (set `self.CurrentBPM` (`self.DiscoBPM`))
        (else
          (`self.GoSport` :!label _label_7)
          (set `self.CurrentBPM` (`self.SportBPM`)))))
    (:`2`
      (if _isfirstteamdisco
        (goto _label_7)
        (else
          (goto _label_6))))))

(event `GoDisco`
  (`AudioComponent.SetSound` (`self.Disco`) (`KismetArrayLibrary.Array_Random` (`self.DiscoMusics`)))
  (`|ExecutionSequence`
    (:`then_0`
      (goto _label_4))
    (:`then_1`
      (goto _label_3 :!via `Reverse`))
    (:`then_2`
      (goto _label_5 :!via `Reverse`))))

(event `GoSport`
  (`AudioComponent.SetSound` (`self.Sport`) (`KismetArrayLibrary.Array_Random` (`self.SportMusics`)))
  (`|ExecutionSequence`
    (:`then_0`
      (goto _label_5))
    (:`then_1`
      (goto _label_4 :!via `Reverse`))
    (:`then_2`
      (goto _label_3 :!via `Reverse`))))

(fn `UserConstructionScript`)