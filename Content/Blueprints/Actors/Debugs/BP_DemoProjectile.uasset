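; BP_DemoProjectile is a debug actor that repeatedly fires a chosen Projectile class for demonstration.
; On BeginPlay, if the class is valid, a looping Delay spawns a new instance every two seconds at the Billboard component's world transform.
; The construction script labels the actor by setting its TextRender to the Projectile class's display name.
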(event `self.ReceiveBeginPlay`
  (bind _projectile (`self.Projectile`))
  (if (`KismetSystemLibrary.IsValidClass` _projectile)
    (`KismetSystemLibrary.Delay` 2.0 :!label _label)
    (`|SpawnActorFromClass` _projectile (`SceneComponent.K2_GetComponentToWorld` (`self.Billboard`)) "Undefined" "MultiplyWithRoot" null null)
    (goto _label)))

(fn `UserConstructionScript`
  (`TextRenderComponent.K2_SetText` (`self.TextRender`) (`KismetTextLibrary.Conv_StringToText` (`KismetSystemLibrary.GetClassDisplayName` (`self.Projectile`)))))