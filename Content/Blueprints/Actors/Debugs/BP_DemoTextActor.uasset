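; BP_DemoTextActor is a debug actor that displays configurable text in the world.
; Its construction script applies the text, color and world size variables to a text render component.
; When RotateTowardsPlayer is set, Tick rotates the root component toward the first player's controlled pawn using a look-at rotation.
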(event `self.ReceiveTick`
  (params (DeltaSeconds :type "Float (single-precision)"))
  (bind _returnvalue (`Controller.K2_GetPawn` (`GameplayStatics.GetPlayerController` 0)))
  (if (`self.RotateTowardsPlayer`)
    (`/Engine/EditorBlueprintResources/StandardMacros.IsValid` _returnvalue
      (:`Is Valid`
        (`SceneComponent.K2_SetWorldRotation` (`self.DefaultSceneRoot`) (`KismetMathLibrary.FindLookAtRotation` (`self.K2_GetActorLocation`) (`self.K2_GetActorLocation` _returnvalue)) false false)))))

(fn `UserConstructionScript`
  (bind _textrender1 (`self.TextRender1`))
  (`TextRenderComponent.K2_SetText` _textrender1 (`KismetTextLibrary.Conv_StringToText` (`self.TextValue`)))
  (`TextRenderComponent.SetTextRenderColor` _textrender1 (`KismetMathLibrary.Conv_LinearColorToColor` (`self.Color`)))
  (`TextRenderComponent.SetWorldSize` _textrender1 (`self.Size`)))