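; BP_Puddle is a puddle actor that shows a material matching its puddle type and plays a player absorption feedback sound when entered.
; On BeginPlay it binds handlers to its puddle-type and enter-puddle dispatchers.
; Setting the type swaps the mesh material from an array indexed by the type enum, and entering plays the sound at the actor's location.
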(event `onEnterPuddle_Event` :!signature `self.onEnterPuddle`
  (params (_actor :type "Actor Object Reference"))
  (`GameplayStatics.PlaySoundAtLocation` "/Game/Audio/Sounds/Player/SA_Player_Feedback_Absorption_MOI.SA_Player_Feedback_Absorption_MOI" (`self.K2_GetActorLocation`) (struct) 1.0 1.0 0.0 null null null null))

(event `self.ReceiveBeginPlay`
  (add `self.onSetPuddleType` (delegate `SetPuddle`))
  (add `self.onEnterPuddle` (delegate `onEnterPuddle_Event`)))

(event `SetPuddle`
  (`PrimitiveComponent.SetMaterial` (`self.mesh`) 0 (`|GetArrayItem` (`self.Texture`) (`KismetMathLibrary.Conv_ByteToInt` (`self.type`)))))

(fn `UserConstructionScript`)