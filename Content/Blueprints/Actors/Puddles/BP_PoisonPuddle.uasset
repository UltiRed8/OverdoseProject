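; BP_PoisonPuddle is a puddle actor whose own logic plays an intermittent ambient sound.
; On BeginPlay it runs the parent logic, then loops: wait a random few seconds, activate the Audio component, wait out the sound's duration, repeat.
; The loop uses latent Delays wired back on themselves instead of Tick.
; Overlap and construction add nothing beyond the parent class.
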(event `self.ReceiveBeginPlay`
  (bind _audio (`self.Audio`))
  (`parent.ReceiveBeginPlay`)
  (`KismetSystemLibrary.Delay` (`KismetMathLibrary.RandomFloatInRange` 2.0 3.0) :!label _label)
  (`ActorComponent.Activate` _audio false)
  (`KismetSystemLibrary.Delay` (`SoundBase.Duration` (`AudioComponent.Sound` _audio)))
  (goto _label))

(fn `UserConstructionScript`
  (`parent.UserConstructionScript`))