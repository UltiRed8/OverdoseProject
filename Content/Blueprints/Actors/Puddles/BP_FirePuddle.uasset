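; BP_FirePuddle is a fire puddle actor that plays recurring sounds from two audio components.
; On BeginPlay it runs the parent logic, then starts two independent loops, one per component.
; Each loop waits a short random delay, activates its audio, waits out the sound's duration and repeats, so the two drift out of sync.
; Overlap and Tick events are disabled, and construction only calls the parent.
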(event `self.ReceiveBeginPlay`
  (bind _audio (`self.Audio`))
  (bind _audio2 (`self.Audio2`))
  (`parent.ReceiveBeginPlay`)
  (`|ExecutionSequence`
    (:`then_0`
      (`KismetSystemLibrary.Delay` (`KismetMathLibrary.RandomFloatInRange` 2.0 3.0) :!label _label)
      (`ActorComponent.Activate` _audio false)
      (`KismetSystemLibrary.Delay` (`SoundBase.Duration` (`AudioComponent.Sound` _audio)))
      (goto _label))
    (:`then_1`
      (`KismetSystemLibrary.Delay` (`KismetMathLibrary.RandomFloatInRange` 2.0 3.0) :!label _label_2)
      (`ActorComponent.Activate` _audio2 false)
      (`KismetSystemLibrary.Delay` (`SoundBase.Duration` (`AudioComponent.Sound` _audio2)))
      (goto _label_2))))

(fn `UserConstructionScript`
  (`parent.UserConstructionScript`))