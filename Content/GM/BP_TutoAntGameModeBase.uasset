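; BP_TutoAntGameModeBase is a game mode, apparently for an ant tutorial, that handles the handover from loading screen to play.
; BeginPlay shows the UI_Loading widget and binds to the LoadingSubsystem's OnLoadingEnded dispatcher.
; When loading ends, it adds the UI_UniquePause widget to the viewport and sets every player controller to game-only input.
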(event `onLoadingEnded_Event`
  (bind _returnvalue (`|CreateWidget` "/Game/Widget/Menu/UI_Player/UI_UniquePause.UI_UniquePause_C"))
  (`UserWidget.AddToViewport` _returnvalue 0)
  (bind _returnvalue_2 (`self.GetNumPlayers`))
  (for _index (range _returnvalue_2)
    (`WidgetBlueprintLibrary.SetInputMode_GameOnly` (`GameplayStatics.GetPlayerController` _index))))

(event `self.ReceiveBeginPlay`
  (bind _returnvalue (`|CreateWidget` "/Game/Widget/Menu/UI_Player/UI_Loading.UI_Loading_C"))
  (`UserWidget.AddToViewport` _returnvalue 0)
  (add `LoadingSubsystem.onLoadingEnded` (subsystem `LoadingSubsystem`) (delegate `onLoadingEnded_Event`)))

(fn `UserConstructionScript`)